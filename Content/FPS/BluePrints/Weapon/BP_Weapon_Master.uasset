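; BP_Weapon_Master is the base FPS hitscan weapon, handling single and automatic fire, damage, ammo and reloading.
; Each shot sphere-traces from the camera with random spread, then re-traces from the SKFMesh muzzle toward that point, with debug drawing.
; ShootInf spends a round and damages hits, while the AutoFireMode macro repeats shots through a gate-and-delay loop.
; Ammo initialisation and reload updates run only on authority, the latter after a sound and short delay.
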(event Custom|OffSweaponFire
  (Utilities|AutoFireMode) ; enters at Close
)

(event Custom|OnWeaponFire
  (switch Utilities|FlowControl|Switch|SwitchonE_FiringMode (Variables|Default|GetFiringMode)
    (:NewEnumerator0
      _)
    (:NewEnumerator1
      (Utilities|AutoFireMode
        (:OUT
          _))))
  (bind (_outhit _returnvalue _fmuzzle _mmuzzle) (CallFunction|SphereTrace))
  (CallFunction|ShootInf _outhit _returnvalue _fmuzzle _mmuzzle))

(event Custom|ShootInf
  (params (Hit%20Result :type Hit%20Result%20Structure%20%28by%20ref%29) (Is%20Hit :type Boolean) (FMuzzle :type Vector) (MMuzzle :type Vector))
  (Variables|Default|SetCurrentAmmoInclip (Math|Integer|Clamp(Integer) (- (Variables|Default|GetCurrentAmmoInclip) 1) 0 (Variables|Default|GetMaxAmmoClipSize)))
  (if Is%20Hit
    (Game|Damage|ApplyDamage (.HitActor (Collision|BreakHitResult Hit%20Result)) 1e+01 (Game|GetInstigatorController) self "/Script/Engine.DamageType")))

(event Custom|OnReloadWeapon
  (CallFunction|ReloadFX)
  (Utilities|FlowControl|Delay 0.2)
  (CallFunction|ReloadAddAmmo))

(event Custom|ReloadFX
  (Audio|SpawnSound2D "/Game/MP_FPSBasic/Audio/Cues/A_Rifle_Reload_Cue.A_Rifle_Reload_Cue" 1.0 1.0 0.0 0))

(event EventBeginPlay
  ;[1 1 1] 총알 지정
  (Networking|SwitchHasAuthority
    (:Authority
      (Variables|Default|SetCurrentMaxAmmo (Variables|Default|GetMaxAmmo))
      (Variables|Default|SetCurrentAmmoInclip (Variables|Default|GetMaxAmmoClipSize)))))

(event Collision|EventActorBeginOverlap
  (params (OtherActor :type Actor%20Object%20Reference)))

(event EventTick
  (params (DeltaSeconds :type Float%20%28single-precision%29)))

(fn ConstructionScript)

(fn SphereTrace
  (bind _returnvalue (Math|Float|MakeLiteralFloat 1.0))
  (bind _returnvalue_2 (Components|GetOwner))
  (bind _returnvalue_3 (Game|GetPlayerCameraManager 0))
  (bind _sk_f_mesh (Variables|Default|GetSK_F_Mesh))
  (bind _returnvalue_4 (Transformation|GetSocketLocation _sk_f_mesh "Muzzle"))
  (bind _returnvalue_5 (Camera|GetCameraLocation _returnvalue_3))
  (bind _array (Utilities|Array|MakeArray _returnvalue_2))
  (bind (_outhit _returnvalue_6) (Collision|SphereTraceByChannel _returnvalue_5 (+ (+ _returnvalue_5 (* (Math|Vector|GetForwardVector (Camera|GetCameraRotation _returnvalue_3)) (Math|Float|MakeLiteralFloat 5e+03))) (* (Math|Random|RandomFloatinRange 0.0 3e+02) (Math|Random|RandomUnitVector))) _returnvalue "TraceTypeQuery1" false _array "ForDuration"))
  (bind (_outhit_2 _returnvalue_7) (Collision|SphereTraceByChannel _returnvalue_4 (select _returnvalue_6 (.ImpactPoint (Collision|BreakHitResult _outhit)) (.TraceEnd (Collision|BreakHitResult _outhit))) _returnvalue "TraceTypeQuery1" false _array "ForDuration"))
  (return _outhit_2 _returnvalue_7 _returnvalue_4 (Transformation|GetSocketLocation (Variables|Default|GetSK_M_Mesh) "Muzzle")))

(fn ReloadAddAmmo
  (Networking|SwitchHasAuthority
    (:Authority
      (bind _output_get (LocalVariables|SetAmmoNeededfor%20Reload (- (Variables|Default|GetCurrentAmmoInclip) (Variables|Default|GetMaxAmmoClipSize))))
      (if (<= (Variables|Default|GetCurrentMaxAmmo) _output_get)
        (Variables|Default|SetCurrentMaxAmmo (+ (Variables|Default|GetCurrentAmmoInclip) (Variables|Default|GetCurrentMaxAmmo)))
        (Variables|Default|SetCurrentMaxAmmo 0)
        (else
          (Variables|Default|SetCurrentMaxAmmo (- (Variables|Default|GetCurrentMaxAmmo) (LocalVariables|GetAmmoNeededfor%20Reload)))
          (Variables|Default|SetCurrentAmmoInclip (Variables|Default|GetMaxAmmoClipSize)))))))