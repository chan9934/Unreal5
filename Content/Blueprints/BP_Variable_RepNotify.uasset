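; Traffic light actor that demonstrates RepNotify variable replication by cycling its lit color.
; The construction script creates a dynamic material instance on the traffic light mesh.
; On BeginPlay, only the authority loops endlessly, switching LightScalar between yellow, red and green values with a delay between each.
; OnRep_LightScalar writes the replicated value into the material's scalar parameter, updating the displayed light.
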(event EventBeginPlay
  (Networking|SwitchHasAuthority :!label _label
    (:Authority
      (Utilities|FlowControl|Delay 1.0)
      (Variables|Default|SetLightScalar (Variables|Default|GetYellowScalar))
      (Utilities|FlowControl|Delay 1.0)
      (Variables|Default|SetLightScalar (Variables|Default|GetRedScalar))
      (Utilities|FlowControl|Delay 1.0)
      (Variables|Default|SetLightScalar (Variables|Default|GetGreenScalar))
      (goto _label))))

(event Collision|EventActorBeginOverlap
  (params (OtherActor :type Actor%20Object%20Reference)))

(event EventTick
  (params (DeltaSeconds :type Float%20%28single-precision%29)))

(fn ConstructionScript
  (bind _returnvalue (Rendering|Material|CreateDynamicMaterialInstance (Variables|Default|GetSM_Traaffic_Light) 1 0 "None" :!class /Script/Engine.PrimitiveComponent))
  (Variables|Default|SetMat _returnvalue))

(fn OnRepLightScalar
  (Rendering|Material|SetScalarParameterValue (Variables|Default|GetMat) (Variables|Default|GetScalarParamName) (Variables|Default|GetLightScalar) :!class /Script/Engine.MaterialInstanceDynamic))